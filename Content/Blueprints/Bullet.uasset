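; Bullet is a Paper2D flipbook projectile that flies along a forward vector until it is marked as hit.
; Tick offsets the capsule by BulletForward times Speed without sweep or delta-time scaling, then swaps between the flight and strike flipbooks.
; The BulletHit event, with no caller in this graph, sets HasHit, which zeroes the offset, and stops active movement.
; The AnimationStateMachine function and axis-locking nodes are present but never run.
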(event Custom|BulletHit
  (Variables|Default|SetHasHit true)
  (Class|NavMovementComponent|StopActiveMovement))

(event Custom|UpdateAnimation
  (if (Variables|Default|GetHasHit)
    (Sprite|SetFlipbook "/Game/Flipbooks/BulletStrike.BulletStrike")
    (else
      (Sprite|SetFlipbook "/Game/Flipbooks/BulletFlip.BulletFlip"))))

(event EventBeginPlay)

(event EventTick
  (params (DeltaSeconds :type Float%20%28single-precision%29))
  (Transformation|AddRelativeLocation (Variables|Collision|GetCapsuleComponent) (* (Variables|Default|GetBulletForward) (* (Math|Conversions|ToInteger(Boolean) (not (Variables|Default|GetHasHit))) (Variables|Default|GetSpeed))) false)
  (CallFunction|UpdateAnimation))

(fn ConstructionScript)

(fn AnimationStateMachine
  (params (hasStruck :type Boolean))
  (if hasStruck
    (LocalVariables|SetAnimationState "NewEnumerator1")
    (else
      (LocalVariables|SetAnimationState "NewEnumerator0")))
  (return (Utilities|Select :Index (LocalVariables|GetAnimationState) :NewEnumerator0 (Variables|Default|GetInFlight) :NewEnumerator1 (Variables|Default|GetStrike))))