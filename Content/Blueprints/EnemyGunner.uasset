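; EnemyGunner is an enemy pawn that patrols back and forth along world X; no firing logic appears here.
; Each Tick it adds movement input toward -X or +X according to the PatrolAEnd and PatrolBEnd flags.
; UpdatePatrolA and UpdatePatrolB compare X to the PatrolA and PatrolB bounds, rechecking only the active leg until it ends.
; The two checks feed into each other, looping while both are false.
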(event Custom|UpdatePatrolB
  (bind _returnvalue (Transformation|GetActorTransform))
  (bind _location (Math|Transform|BreakTransform _returnvalue))
  (bind _x (Math|Vector|BreakVector _location))
  (bind _output_get (Variables|Default|SetPatrolBEnd (< _x (Math|Conversions|ToFloat(Integer) (Variables|Default|GetPatrolB))) :!label _label))
  (if (not _output_get)
    (bind _output_get_2 (Variables|Default|SetPatrolAEnd (> _x (Math|Conversions|ToFloat(Integer) (Variables|Default|GetPatrolA)))))
    (if (not _output_get_2)
      (goto _label))))

(event Custom|UpdatePatrolA
  (bind _returnvalue (Transformation|GetActorTransform))
  (bind _location (Math|Transform|BreakTransform _returnvalue))
  (bind _x (Math|Vector|BreakVector _location))
  (bind _output_get (Variables|Default|SetPatrolAEnd (> _x (Math|Conversions|ToFloat(Integer) (Variables|Default|GetPatrolA))) :!label _label))
  (if (not _output_get)
    (bind _output_get_2 (Variables|Default|SetPatrolBEnd (< _x (Math|Conversions|ToFloat(Integer) (Variables|Default|GetPatrolB)))))
    (if (not _output_get_2)
      (goto _label))))

(event EventBeginPlay)

(event EventActorBeginOverlap
  (params (OtherActor :type Actor%20Object%20Reference)))

(event EventTick
  (params (DeltaSeconds :type Float%20%28single-precision%29))
  (if (Variables|Default|GetPatrolAEnd)
    (Pawn|Input|AddMovementInput "-1.000000, 0, 0" 1.0 false)
    (CallFunction|UpdatePatrolA)
    (elif (Variables|Default|GetPatrolBEnd)
      (Pawn|Input|AddMovementInput "1.000000, 0, 0" 1.0 false)
      (CallFunction|UpdatePatrolB))))

(fn ConstructionScript)