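; A Paper2D bullet actor that flies along its forward vector and plays a strike animation when it hits something.
; Each Tick moves it by Speed without sweep or delta-time scaling until the Hit event sets HasHit.
; Tick then switches the flipbook to a non-looping BulletStrike, and the actor destroys itself when that flipbook finishes playing.
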(event OnFinishedPlaying(RenderComponent)
  (if (Variables|Default|GetHasHit)
    (Actor|DestroyActor)))

(event Custom|Hit
  (Variables|Default|SetHasHit true))

(event EventBeginPlay)

(event EventTick
  (params (DeltaSeconds :type Float%20%28single-precision%29))
  (if (Variables|Default|GetHasHit)
    (Sprite|SetFlipbook "/Game/Flipbooks/BulletStrike.BulletStrike")
    (Components|Timeline|SetLooping false)
    (else
      (Transformation|AddRelativeLocation (* (Math|Vector|GetForwardVector) (Variables|Default|GetSpeed)) false))))

(fn ConstructionScript)