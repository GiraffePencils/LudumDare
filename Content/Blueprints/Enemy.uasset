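; Enemy pawn that patrols back and forth along world X, fires back when damaged and destroys itself when health drops below zero.
; Each tick runs a forward pawn line trace, storing Hit without acting on it here, then moves the enemy.
; PatrolA/PatrolB bounds set direction flags and turn it around; the health check runs within movement.
; Damage triggers a Bullet spawn along actor forward, ignoring the target argument.
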(event Custom|TakeDamage
  (params (Damage :type Float%20%28single-precision%29))
  (Variables|Default|SetHealth (- (Variables|Default|GetHealth) Damage))
  (CallFunction|ShootPlayer))

(event Custom|ShootPlayer
  (CallFunction|ShootGun "0, 0, 0"))

(event EventTick
  (params (DeltaSeconds :type Float%20%28single-precision%29))
  (|RayCast)
  (|MoveEnemy))

(fn ConstructionScript)

(fn TakeDamageFunc
  (params (Damage :type Float%20%28single-precision%29 :default 0.0))
  (Variables|Default|SetHealth (- (Variables|Default|GetHealth) Damage)))

(fn ShootGun
  (params (Target :type Vector))
  (bind _returnvalue (Game|SpawnActorfromClass "/Game/Blueprints/Bullet.Bullet_C" (Transformation|GetActorTransform) true (Transformation|GetActorForwardVector) (Variables|Default|GetBulletSpeed) self))
  (return _returnvalue))

(event Custom|UpdatePatrolA
  (bind _output_get (Variables|Default|SetPatrolAEnd (> (.X (Math|Vector|BreakVector (.Location (Math|Transform|BreakTransform (Transformation|GetActorTransform))))) (Math|Conversions|ToFloat(Integer) (Variables|Default|GetPatrolA)))))
  (if (not _output_get)
    (Transformation|AddLocalRotation (Variables|Collision|GetCapsuleComponent) (Class|KismetMathLibrary|MakeRot 0.0 1.8e+02 0.0) false)
    (CallFunction|UpdatePatrolB)))

(event Custom|UpdatePatrolB
  (bind _output_get (Variables|Default|SetPatrolBEnd (< (.X (Math|Vector|BreakVector (.Location (Math|Transform|BreakTransform (Transformation|GetActorTransform))))) (Math|Conversions|ToFloat(Integer) (Variables|Default|GetPatrolB)))))
  (if (not _output_get)
    (Transformation|AddLocalRotation (Variables|Collision|GetCapsuleComponent) (Class|KismetMathLibrary|MakeRot 0.0 1.8e+02 0.0) false)
    (CallFunction|UpdatePatrolA)))