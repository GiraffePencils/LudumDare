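; Paper2D player character for a side-scroller with depth lanes, melee attack and health.
; Input drives left/right movement with facing flips, jumping and stepped Y-axis lane changes, with offsets inverted to match facing.
; The movement axis event and attack click refresh the flipbook through a function-based idle/run/jump/attack state selector.
; Clicking damages overlapping enemies, overlapping bullets damage the player, and death destroys the actor and reopens LevelOne.
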(event OnComponentBeginOverlap(CapsuleComponent)
  (params (OtherActor :type Actor%20Object%20Reference) (OtherComp :type Primitive%20Component%20Object%20Reference) (OtherBodyIndex :type Integer) (bFromSweep :type Boolean) (SweepResult :type Hit%20Result%20Structure%20%28by%20ref%29))
  (for _array_element (Collision|GetOverlappingActors "/Game/Blueprints/BulletBP.BulletBP_C" :!class /Script/Engine.PrimitiveComponent)
    (bind _asbullet_bp (Utilities|Casting|CastToBulletBP _array_element))
    (Default|Hit _asbullet_bp)
    (Game|Damage|ApplyPointDamage self 5.0 (Math|Vector|GetForwardVector _asbullet_bp) (Variables|Default|GetIBeenShot) 0 _array_element "/Script/Engine.DamageType")))

(event Custom|UpdateAnimation
  (Variables|Default|SetisMoving (> (Math|Vector|VectorLength (Transformation|GetVelocity)) 0.0))
  (Variables|Default|SetisFalling (AI|Components|NavMovement|IsFalling (Variables|Character|GetCharacterMovement)))
  (bind _outputflipbook (CallFunction|AnimationStateMachine (Variables|Default|GetisFalling) (Variables|Default|GetisMoving) (Variables|Default|GetIsAttacking)))
  (Sprite|SetFlipbook (Variables|Default|GetSprite) _outputflipbook)
  (Audio|Components|Audio|Play))

(event EventBeginPlay)

(event EventTick
  (params (DeltaSeconds :type Float%20%28single-precision%29)))

(event EventAnyDamage
  (params (Damage :type Float%20%28single-precision%29) (DamageType :type Damage%20Type%20Object%20Reference) (InstigatedBy :type Controller%20Object%20Reference) (DamageCauser :type Actor%20Object%20Reference))
  (CallFunction|TakeDamage Damage)
  (if (< (Variables|Default|GetHealth) 0.0)
    (Actor|DestroyActor)))

(event EventDestroyed
  (if (not (> (Variables|Default|GetHealth) 0.0))
    (Game|OpenLevel(byName) "LevelOne")))

(event Input|ActionEvents|InputActionMouseLeftClick
  (:Pressed
    (Variables|Default|SetIsAttacking true)
    (Components|Timeline|SetLooping false)
    (CallFunction|UpdateAnimation)
    (for _array_element (Collision|GetOverlappingActors "/Game/Blueprints/Enemy.Enemy_C" :!class /Script/Engine.PrimitiveComponent)
      (bind _asenemy (Utilities|Casting|CastToEnemy _array_element))
      (Game|Damage|ApplyPointDamage _asenemy (Variables|Default|GetDamage) (Math|Vector|GetForwardVector) (Variables|Default|GetIHitTheGuy) 0 self "/Script/Engine.DamageType")))
  (:Released
    (Components|Timeline|SetLooping (Variables|Default|GetSprite) true)
    (Variables|Default|SetIsAttacking false)))

(event Input|ActionEvents|InputActionJump
  (:Pressed
    (Character|Jump)))

(fn ConstructionScript
  (bind _aspaper_flipbook_component (Utilities|Casting|CastToPaperFlipbookComponent (Variables|Animations|GetattackFlipbook)))
  (Components|Timeline|SetLooping _aspaper_flipbook_component false))

(fn AnimationStateMachine
  (params (isFalling :type Boolean :default false) (isMoving :type Boolean :default false) (isAttacking :type Boolean :default false))
  (LocalVariables|SetisAttackingLocal isAttacking)
  (LocalVariables|SetisFallingLocal isFalling)
  (LocalVariables|SetisMovingLocal isMoving)
  (if (LocalVariables|GetisFallingLocal)
    (LocalVariables|SetAnimationState "NewEnumerator2")
    (elif (LocalVariables|GetisMovingLocal)
      (LocalVariables|SetAnimationState "NewEnumerator1")
      (else
        (LocalVariables|SetAnimationState "NewEnumerator0"))))
  (if (LocalVariables|GetisAttackingLocal)
    (LocalVariables|SetAnimationState "NewEnumerator3"))
  (return (Utilities|Select :Index (LocalVariables|GetAnimationState) :NewEnumerator0 (Variables|Animations|GetidleFlipbook) :NewEnumerator1 (Variables|Animations|GetrunFlipbook) :NewEnumerator2 (Variables|Animations|GetjumpFlipbook) :NewEnumerator3 (Variables|Animations|GetattackFlipbook))))

(fn TakeDamage
  (params (Damage :type Float%20%28single-precision%29 :default 0.0))
  (Variables|Default|SetHealth (- (Variables|Default|GetHealth) Damage)))

(event Input|ActionEvents|InputActionToBackground
  (:Pressed
    (if (> (.Y (Math|Vector|BreakVector (Transformation|GetActorLocation))) -5e+02)
      (Transformation|SetRelativeLocationAndRotation (Math|Transform|TransformLocation (Transformation|GetActorTransform) (Variables|Default|GetBackgroundMovement)) "0, 0, 0" false))))

(event Input|ActionEvents|InputActionToForground
  (:Pressed
    (if (< (.Y (Math|Vector|BreakVector (Transformation|GetActorLocation))) 5e+02)
      (Transformation|SetRelativeLocationAndRotation (Variables|Collision|GetCapsuleComponent) (Math|Transform|TransformLocation (Transformation|GetActorTransform) (Variables|Default|GetForgroundMovement)) "0, 0, 0" false))))

(event Input|AxisEvents|InputAxisMoveRight
  (params (AxisValue :type Float%20%28single-precision%29))
  (Pawn|Input|AddMovementInput "1.000000, 0, 0" AxisValue false)
  (CallFunction|UpdateAnimation)
  (Math|Float|CompareFloat AxisValue 0.0
    (:>
      (Pawn|SetControlRotation (Pawn|GetController) (Class|KismetMathLibrary|MakeRot 0.0 0.0 0.0))
      (Variables|Default|SetForgroundMovement "0,500.000000, 0")
      (Variables|Default|SetBackgroundMovement "0,-500.000000, 0"))
    (:<
      (Pawn|SetControlRotation (Pawn|GetController) (Class|KismetMathLibrary|MakeRot 0.0 1.8e+02 0.0))
      (Variables|Default|SetForgroundMovement "0,-500.000000, 0")
      (Variables|Default|SetBackgroundMovement "0,500.000000, 0"))))